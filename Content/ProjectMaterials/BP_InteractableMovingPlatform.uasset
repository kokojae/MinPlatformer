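; BP_InteractableMovingPlatform is a platform that moves between two points each time it is interacted with.
; BeginPlay caches the world locations of MovingPlatform and MovingPlatformEnd as the start and end positions.
; Interact calls Move and returns true; Move uses a FlipFlop to alternately play and reverse the PlatformTime timeline.
; The timeline's float track drives a Lerp that sets the platform's world location, without sweeping.
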(event `self.ReceiveBeginPlay`
  (set `self.StartLocation` (`SceneComponent.K2_GetComponentLocation` (`self.MovingPlatform`)))
  (set `self.EndLocation` (`SceneComponent.K2_GetComponentLocation` (`self.MovingPlatformEnd`))))

(event `Move`
  (`/Engine/EditorBlueprintResources/StandardMacros.FlipFlop`
    (:`A`
      (bind (_direction _platformfloattime) (`Timeline|PlatformTime` :!label _label)
        (:`Update`
          (`SceneComponent.K2_SetWorldLocation` (`self.MovingPlatform`) (`KismetMathLibrary.VLerp` (`self.StartLocation`) (`self.EndLocation`) _platformfloattime) false false))))
    (:`B`
      (goto _label :!via `Reverse`))))

(fn `Interact`
  (returns (Success :type Boolean))
  (`self.Move`)
  (return true))

(fn `UserConstructionScript`)