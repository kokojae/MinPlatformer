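; BP_TriggerDoor is a door that slides vertically when interacted with.
; A box trigger shows a text render while a ThirdPersonCharacter overlaps it and hides it when the overlap ends.
; Interact calls OpenDoor, whose timeline adds a Z offset to the mesh's world location saved at BeginPlay.
; The timeline only plays forward, with no closing logic.
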(event `self.ReceiveBeginPlay`
  (set `self.Starting Location` (`SceneComponent.K2_GetComponentLocation` (`self.StaticMeshComponent`))))

(event `self.Box.OnComponentBeginOverlap`
  (params (OverlappedComponent :type "PrimitiveComponent Object Reference") (OtherActor :type "Actor Object Reference") (OtherComp :type "PrimitiveComponent Object Reference") (OtherBodyIndex :type Integer) (bFromSweep :type Boolean) (SweepResult :type "HitResult Structure (by ref)"))
  (cast `/Game/ThirdPersonBP/Blueprints/ThirdPersonCharacter` OtherActor)
  (`SceneComponent.SetVisibility` (`self.TextRender`) true false))

(event `self.Box.OnComponentEndOverlap`
  (params (OverlappedComponent :type "PrimitiveComponent Object Reference") (OtherActor :type "Actor Object Reference") (OtherComp :type "PrimitiveComponent Object Reference") (OtherBodyIndex :type Integer))
  (cast `/Game/ThirdPersonBP/Blueprints/ThirdPersonCharacter` OtherActor)
  (`SceneComponent.SetVisibility` (`self.TextRender`) false false))

(event `Open Door`
  (bind (_direction `_새_트랙_0`) (`Timeline|Timeline`)
    (:`Update`
      (`SceneComponent.K2_SetWorldLocation` (`self.StaticMeshComponent`) (+ (`self.Starting Location`) (`KismetMathLibrary.MakeVector` 0.0 0.0 `_새_트랙_0`)) false false))))

(fn `Interact`
  (returns (Success :type Boolean))
  (`self.Open Door`)
  (return false))

(fn `UserConstructionScript`)