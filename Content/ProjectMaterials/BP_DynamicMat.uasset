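; BP_DynamicMat is an actor demonstrating runtime material changes on a static mesh with a trigger box.
; On BeginPlay it creates and stores a dynamic instance of DynamicMatGlow, colors its GlowOrbColor parameter green and applies it to the mesh.
; When a ThirdPersonCharacter enters the trigger, it sets a black vector value, but the parameter name is left as None, so GlowOrbColor is not targeted.
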(event `self.ReceiveBeginPlay`
  (bind _returnvalue (`PrimitiveComponent.CreateDynamicMaterialInstance` (`self.StaticMesh`) 0 "/Game/ProjectMaterials/DynamicMatGlow.DynamicMatGlow" "None"))
  (bind _output_get (set `self.OurDynamicMaterial` _returnvalue))
  (`MaterialInstanceDynamic.SetVectorParameterValue` _output_get "GlowOrbColor" (struct :`G` 1.0 :`A` 1.0))
  (`PrimitiveComponent.SetMaterial` (`self.StaticMesh`) 0 (`self.OurDynamicMaterial`)))

(event `self.TriggerBox.OnComponentBeginOverlap`
  (params (OverlappedComponent :type "PrimitiveComponent Object Reference") (OtherActor :type "Actor Object Reference") (OtherComp :type "PrimitiveComponent Object Reference") (OtherBodyIndex :type Integer) (bFromSweep :type Boolean) (SweepResult :type "HitResult Structure (by ref)"))
  (cast `/Game/ThirdPersonBP/Blueprints/ThirdPersonCharacter` OtherActor)
  (`MaterialInstanceDynamic.SetVectorParameterValue` :`self` (`self.OurDynamicMaterial`)))

(fn `UserConstructionScript`)